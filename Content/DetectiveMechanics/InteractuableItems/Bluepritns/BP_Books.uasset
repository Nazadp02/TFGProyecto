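; BP_Books is a book combination puzzle that opens a wall once all of its books are in the completed state.
; Tick, throttled by a Delay, calls CheckCompletedCombination, which ANDs CurrentCompletedBooks from six BP_TrueBook child actors.
; When the check passes, MoveWall runs after a short delay, and a Timeline lerps WallMesh downward in relative space.
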(event Custom|MoveWall
  ;[1 1 1] ACTIVAR MOVIMIENTO DE PARED
  (bind _alpha (Timeline|Timeline Play)
    (:Update
      (Transformation|SetRelativeLocation (Variables|Default|GetWallMesh) (Math|Vector|Lerp(Vector) "12.000000,-278.000000,64.000000" "12.000000,-278.000000,-500.000000" _alpha) false false))))

(event EventTick
  (params (DeltaSeconds :type Float%20%28single-precision%29))
  (Utilities|FlowControl|Delay 1.0)
  (bind _combomatch_ (CallFunction|CheckCompletedCombination))
  (if _combomatch_
    (Utilities|FlowControl|Delay 1.0)
    (CallFunction|MoveWall)))

(fn ConstructionScript)

(fn CheckCompletedCombination
  (return (== (Class|KismetMathLibrary|AndIntInt (Variables|/Game/DetectiveMechanics/InteractuableItems/Bluepritns/BP_TrueBook.BP_TrueBook_C|GetCurrentCompletedBooks (.AsBP%20True%20Book (Utilities|Casting|CastToBP_TrueBook (Variables|/Script/Engine.ChildActorComponent|GetChildActor (Variables|Default|GetBP_TrueBook))))) (Variables|/Game/DetectiveMechanics/InteractuableItems/Bluepritns/BP_TrueBook.BP_TrueBook_C|GetCurrentCompletedBooks (.AsBP%20True%20Book (Utilities|Casting|CastToBP_TrueBook (Variables|/Script/Engine.ChildActorComponent|GetChildActor (Variables|Default|GetBP_TrueBook1))))) (Variables|/Game/DetectiveMechanics/InteractuableItems/Bluepritns/BP_TrueBook.BP_TrueBook_C|GetCurrentCompletedBooks (.AsBP%20True%20Book (Utilities|Casting|CastToBP_TrueBook (Variables|/Script/Engine.ChildActorComponent|GetChildActor (Variables|Default|GetBP_TrueBook2))))) (Variables|/Game/DetectiveMechanics/InteractuableItems/Bluepritns/BP_TrueBook.BP_TrueBook_C|GetCurrentCompletedBooks (.AsBP%20True%20Book (Utilities|Casting|CastToBP_TrueBook (Variables|/Script/Engine.ChildActorComponent|GetChildActor (Variables|Default|GetBP_TrueBook3))))) (Variables|/Game/DetectiveMechanics/InteractuableItems/Bluepritns/BP_TrueBook.BP_TrueBook_C|GetCurrentCompletedBooks (.AsBP%20True%20Book (Utilities|Casting|CastToBP_TrueBook (Variables|/Script/Engine.ChildActorComponent|GetChildActor (Variables|Default|GetBP_TrueBook4))))) (Variables|/Game/DetectiveMechanics/InteractuableItems/Bluepritns/BP_TrueBook.BP_TrueBook_C|GetCurrentCompletedBooks (.AsBP%20True%20Book (Utilities|Casting|CastToBP_TrueBook (Variables|/Script/Engine.ChildActorComponent|GetChildActor (Variables|Default|GetBP_TrueBook5)))))) 1)))