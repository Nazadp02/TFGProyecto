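; BP_Maletin is an interactable briefcase that opens when its four-tumbler combination lock shows the correct code.
; BeginPlay optionally randomizes the four BP_Codigo child-actor tumblers.
; Tick polls through a one-second Delay, with CheckCombination joining the tumbler numbers into a string to compare against Combination.
; A match clears LockedState once and, after a short pause, calls Unlock, whose timeline swings the lid open along its roll axis.
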(event Custom|Unlock
  ;[0.2292 0.2292 0.2292 0.8] DESBLOQUEO DEL MALETIN
  (bind _alpha (Timeline|UnlockMaletin Play)
    (:Update
      (Transformation|SetRelativeRotation (Variables|Default|GetMaletinParteArribaMesh) (Math|Rotator|MakeRotator (* _alpha (Variables|Default|GetRotationAmount)) 0.0 0.0) false false))))

(event EventTick
  (params (DeltaSeconds :type Float%20%28single-precision%29))
  ;[1 1 1] checkea si el codigo es el correcto
  (Utilities|FlowControl|Delay 1.0)
  (bind _combomatch_ (CallFunction|CheckCombination))
  (if _combomatch_
    (Utilities|FlowControl|DoOnce false
      (:Completed
        (Variables|Default|SetLockedState false)
        (Utilities|FlowControl|Delay 0.5)
        (CallFunction|Unlock)
        (Utilities|FlowControl|Delay 2.0)))))

(event EventBeginPlay
  (if (Variables|Default|GetRandomizeTumblerRotation?)
    (Default|RandomnizeTumbler (.AsBP%20Codigo (Utilities|Casting|CastToBP_Codigo (Variables|/Script/Engine.ChildActorComponent|GetChildActor (Variables|Default|GetBP_Codigo1)))))
    (Default|RandomnizeTumbler (.AsBP%20Codigo (Utilities|Casting|CastToBP_Codigo (Variables|/Script/Engine.ChildActorComponent|GetChildActor (Variables|Default|GetBP_Codigo2)))))
    (Default|RandomnizeTumbler (.AsBP%20Codigo (Utilities|Casting|CastToBP_Codigo (Variables|/Script/Engine.ChildActorComponent|GetChildActor (Variables|Default|GetBP_Codigo3)))))
    (Default|RandomnizeTumbler (.AsBP%20Codigo (Utilities|Casting|CastToBP_Codigo (Variables|/Script/Engine.ChildActorComponent|GetChildActor (Variables|Default|GetBP_Codigo4)))))))

(fn ConstructionScript)

(fn CheckCombination
  (return (Utilities|Enum|Equal(Enum) (Variables|Default|GetCombination) (Utilities|String|Append (Utilities|String|ToString(Integer) (Variables|/Game/DetectiveMechanics/InteractuableItems/Bluepritns/BP_Codigo.BP_Codigo_C|GetTumblerNumber (.AsBP%20Codigo (Utilities|Casting|CastToBP_Codigo (Variables|/Script/Engine.ChildActorComponent|GetChildActor (Variables|Default|GetBP_Codigo1)))))) (Utilities|String|ToString(Integer) (Variables|/Game/DetectiveMechanics/InteractuableItems/Bluepritns/BP_Codigo.BP_Codigo_C|GetTumblerNumber (.AsBP%20Codigo (Utilities|Casting|CastToBP_Codigo (Variables|/Script/Engine.ChildActorComponent|GetChildActor (Variables|Default|GetBP_Codigo2)))))) (Utilities|String|ToString(Integer) (Variables|/Game/DetectiveMechanics/InteractuableItems/Bluepritns/BP_Codigo.BP_Codigo_C|GetTumblerNumber (.AsBP%20Codigo (Utilities|Casting|CastToBP_Codigo (Variables|/Script/Engine.ChildActorComponent|GetChildActor (Variables|Default|GetBP_Codigo3)))))) (Utilities|String|ToString(Integer) (Variables|/Game/DetectiveMechanics/InteractuableItems/Bluepritns/BP_Codigo.BP_Codigo_C|GetTumblerNumber (.AsBP%20Codigo (Utilities|Casting|CastToBP_Codigo (Variables|/Script/Engine.ChildActorComponent|GetChildActor (Variables|Default|GetBP_Codigo4))))))))))