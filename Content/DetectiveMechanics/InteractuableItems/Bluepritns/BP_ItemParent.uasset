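; Base detective item that shows a pickup prompt and can be picked up, inspected or dropped.
; Interacting attaches it to the player's grip, or starts inspection if an item is already held.
; Inspection swaps the HUD for a description widget and hands input to the item for mouse rotation and wheel zoom along the camera's view.
; Dropping restores physics in front of the camera; PlaceItem is empty, its pressure-plate attach logic unconnected.
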(event Input|EnhancedActionEvents|EnhancedInputActionIA_InspectionRotate
  (params (ActionValue :type Boolean) (ElapsedSeconds :type Float%20%28double-precision%29) (TriggeredSeconds :type Float%20%28double-precision%29) (InputAction :type Input%20Action%20Object%20Reference :default "/Game/DetectiveMechanics/Inputs/Actions/IA_InspectionRotate.IA_InspectionRotate"))
  ;[1 1 1] Empezar a rotar el objeto en inspeccionar
  (:Started
    (Variables|Default|SetIsRotating true))
  (:Completed
    (Variables|Default|SetIsRotating false)))

(event Input|EnhancedActionEvents|EnhancedInputActionIA_CancelInteraction
  (params (ActionValue :type Boolean) (ElapsedSeconds :type Float%20%28double-precision%29) (TriggeredSeconds :type Float%20%28double-precision%29) (InputAction :type Input%20Action%20Object%20Reference :default "/Game/DetectiveMechanics/Inputs/Actions/IA_CancelInteraction.IA_CancelInteraction"))
  ;[1 1 1] Dejar de inspeccionar
  (:Started
    (CallFunction|StopInspect)))

(event EventLookat
  (params (PlayerCharacter :type BP%20Detective%20Object%20Reference))
  ;[1 1 1] Para que aparezca un mensaje
  (Default|UpdateMessage (Variables|/Game/DetectiveMechanics/DetectiveBlueprints/BP_Detective.BP_Detective_C|GetHUD PlayerCharacter) (Utilities|Text|FormatText "Press E to Pick Up {name}" (Variables|Default|GetItemName))))

(event EventInteractwith
  (params (PlayerCharacter :type BP%20Detective%20Object%20Reference))
  ;[1 1 1] Empezar a inspeccionar el objeto
  (bind _output_get (Variables|Default|SetPlayer%20Character PlayerCharacter))
  (Variables|/Game/DetectiveMechanics/DetectiveBlueprints/BP_Detective.BP_Detective_C|GetCurrentHeldItem _output_get
    (:then
      (CallFunction|StartInspect))
    (:else
      (CallFunction|PickUpItem))))

(event Input|MouseEvents|MouseX
  (params (AxisValue :type Float%20%28single-precision%29))
  ;[1 1 1] Rotación en el modo inspeccionar en x
  (if (Variables|Default|GetIsRotating)
    (Transformation|SetActorRotation (Math|Rotator|CombineRotators (Transformation|GetActorRotation) (Math|Rotator|MakeRotator 0.0 0.0 (* AxisValue -5.0))))))

(event Input|MouseEvents|MouseY
  (params (AxisValue :type Float%20%28single-precision%29))
  ;[1 1 1] Rotación en el modo inspeccionar en y
  (if (Variables|Default|GetIsRotating)
    (Transformation|SetActorRotation (Math|Rotator|CombineRotators (Transformation|GetActorRotation) (Math|Rotator|MakeRotator 0.0 (* AxisValue -5.0) 0.0)))))

(event Input|MouseEvents|MouseWheelDown
  (params (Key :type Key%20Structure))
  (bind _returnvalue (Game|GetPlayerCameraManager 0))
  ;[1 1 1] Más zoom
  (:Pressed
    (bind _output_get (Variables|Default|SetZoomLvl (Math|Integer|Clamp(Integer) (+ (Variables|Default|GetZoomLvl) 1) 1 20)))
    (if (< _output_get 20)
      (Transformation|SetActorLocation (+ (Camera|GetCameraLocation _returnvalue) (* (Math|Vector|GetForwardVector (Camera|GetCameraRotation _returnvalue)) (* (Variables|Default|GetZoomLvl) 2e+01))) false false))))

(event Input|MouseEvents|MouseWheelUp
  (params (Key :type Key%20Structure))
  (bind _returnvalue (Game|GetPlayerCameraManager 0))
  ;[1 1 1] Menos zoom
  (:Pressed
    (bind _output_get (Variables|Default|SetZoomLvl (Math|Integer|Clamp(Integer) (- (Variables|Default|GetZoomLvl) 1) 1 20)))
    (if (> _output_get 1)
      (Transformation|SetActorLocation (+ (Camera|GetCameraLocation _returnvalue) (* (Math|Vector|GetForwardVector (Camera|GetCameraRotation _returnvalue)) (* (Variables|Default|GetZoomLvl) 2e+01))) false false))))

(fn ConstructionScript)

(fn PickUpItem
  (bind _staticmesh (Variables|Default|GetStaticMesh))
  (Transformation|AttachComponentToComponent (Variables|/Game/DetectiveMechanics/DetectiveBlueprints/BP_Detective.BP_Detective_C|GetItemGrip (Variables|Default|GetPlayer%20Character)) "None" "SnapToTarget" "SnapToTarget" "KeepRelative" true)
  (Physics|SetSimulatePhysics _staticmesh false)
  (Collision|SetCollisionEnabled _staticmesh "NoCollision")
  (Variables|/Game/DetectiveMechanics/DetectiveBlueprints/BP_Detective.BP_Detective_C|SetCurrentHeldItem (Variables|Default|GetPlayer%20Character) self))

(fn StartInspect
  (bind _returnvalue (Game|GetPlayerController 0))
  (bind _returnvalue_2 (Game|GetPlayerCameraManager 0))
  (Widget|SetVisibility (Variables|/Game/DetectiveMechanics/DetectiveBlueprints/BP_Detective.BP_Detective_C|GetHUD (Variables|Default|GetPlayer%20Character)) "Hidden")
  (bind _returnvalue_3 (UserInterface|CreateWidget "/Game/DetectiveMechanics/UI/WBP_InspectionMenu.WBP_InspectionMenu_C" 0 (Variables|Default|GetItemDescription)))
  (bind _output_get (Variables|Default|SetInspectionUI _returnvalue_3))
  (UserInterface|Viewport|AddtoViewport _output_get 0)
  (Input|DisableInput (Variables|Default|GetPlayer%20Character) _returnvalue)
  (Input|EnableInput _returnvalue)
  (Transformation|SetActorLocation (+ (Camera|GetCameraLocation _returnvalue_2) (* (Math|Vector|GetForwardVector (Camera|GetCameraRotation _returnvalue_2)) 2e+02)) false false))

(fn StopInspect
  (bind _returnvalue (Game|GetPlayerController 0))
  (Input|DisableInput _returnvalue)
  (Input|EnableInput (Variables|Default|GetPlayer%20Character) _returnvalue)
  (Transformation|SetActorRelativeLocation "0, 0, 0")
  (Transformation|SetActorRelativeRotation "0, 0, 0")
  (Widget|RemovefromParent (Variables|Default|GetInspectionUI))
  (Widget|SetVisibility (Variables|/Game/DetectiveMechanics/DetectiveBlueprints/BP_Detective.BP_Detective_C|GetHUD (Variables|Default|GetPlayer%20Character)) "Visible"))

(fn DropItem
  (bind _returnvalue (Game|GetPlayerCameraManager 0))
  (bind _staticmesh (Variables|Default|GetStaticMesh))
  (Transformation|DetachFromActor "KeepWorld" "KeepWorld" "KeepWorld")
  (Transformation|SetActorLocation (+ (Camera|GetCameraLocation _returnvalue) (* (Math|Vector|GetForwardVector (Camera|GetCameraRotation _returnvalue)) 2e+02)) false false)
  (Physics|SetSimulatePhysics _staticmesh true)
  (Collision|SetCollisionEnabled _staticmesh "QueryAndPhysics"))

(fn PlaceItem)