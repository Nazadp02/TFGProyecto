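; BP_Codigo is a single rotating tumbler of a numeric code lock, showing a digit from 0 to 9.
; SpinTumbler and SpinTumblerBackward play timelines that roll the mesh, guarded by IsTumblerMoving and resettable DoOnce nodes, then wrap the rotation at a full turn.
; NumberCheck maps the truncated angle, in 36-degree steps either way, to TumblerNumber, which is debug-printed after each spin.
; RandomnizeTumbler sets a random starting angle from RandomRotations.
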(event Custom|SpinTumblerBackward
  ;[1 1 1] Girar las piezas
  (if (not (Variables|Default|GetIsTumblerMoving?))
    (Utilities|FlowControl|DoOnce false
      (:Completed
        (Variables|Default|SetIsTumblerMoving? true)
        (bind _alpha (Timeline|TurnBackward PlayFromStart)
          (:Update
            (Transformation|SetRelativeRotation (Variables|Default|GetTumblerMesh) (Math|Rotator|MakeRotator (- (Variables|Default|GetTumblerRotation) _alpha) 0.0 0.0) false false))
          (:Finished
            (Variables|Default|SetTumblerRotation (- (Variables|Default|GetTumblerRotation) _alpha))
            (CallFunction|NumberCheck)
            (CallFunction|ShowTumblerNumber)
            (CallFunction|SpinTumblerBackwardReset)
            (Variables|Default|SetIsTumblerMoving? false)
            (if (<= (Variables|Default|GetTumblerRotation) -3.6e+02)
              (Variables|Default|SetTumblerRotation 0.0))))))))

(event Custom|SpinTumblerBackwardReset
  ;[1 1 1] Girar las piezas
  (Utilities|FlowControl|DoOnce false) ; enters at Reset
)

(event Custom|ShowTumblerNumber
  (Development|PrintString (Utilities|String|Append "Tumbler Number :" (Utilities|String|ToString(Integer) (Variables|Default|GetTumblerNumber)))))

(event Custom|SpinTumbler
  ;[1 1 1] Girar las piezas
  (if (not (Variables|Default|GetIsTumblerMoving?))
    (Utilities|FlowControl|DoOnce false
      (:Completed
        (Variables|Default|SetIsTumblerMoving? true)
        (bind _alpha (Timeline|TurnForward PlayFromStart)
          (:Update
            (Transformation|SetRelativeRotation (Variables|Default|GetTumblerMesh) (Math|Rotator|MakeRotator (+ (Variables|Default|GetTumblerRotation) _alpha) 0.0 0.0) false false))
          (:Finished
            (Variables|Default|SetTumblerRotation (+ (Variables|Default|GetTumblerRotation) _alpha))
            (CallFunction|NumberCheck)
            (CallFunction|ShowTumblerNumber)
            (CallFunction|SpinTumblerReset)
            (Variables|Default|SetIsTumblerMoving? false)
            (if (>= (Variables|Default|GetTumblerRotation) 3.6e+02)
              (Variables|Default|SetTumblerRotation 0.0))))))))

(event Custom|SpinTumblerReset
  ;[1 1 1] Girar las piezas
  (Utilities|FlowControl|DoOnce false) ; enters at Reset
)

(fn ConstructionScript)

(fn NumberCheck
  ;[1 1 1] hacia delante
  (if (== (Math|Float|Truncate (Variables|Default|GetTumblerRotation)) 0)
    (Variables|Default|SetTumblerNumber 0)
    (elif (== (Math|Float|Truncate (Variables|Default|GetTumblerRotation)) 36)
      (Variables|Default|SetTumblerNumber 1)
      (elif (== (Math|Float|Truncate (Variables|Default|GetTumblerRotation)) 72)
        (Variables|Default|SetTumblerNumber 2)
        (elif (== (Math|Float|Truncate (Variables|Default|GetTumblerRotation)) 108)
          (Variables|Default|SetTumblerNumber 3)
          (elif (== (Math|Float|Truncate (Variables|Default|GetTumblerRotation)) 144)
            (Variables|Default|SetTumblerNumber 4)
            (elif (== (Math|Float|Truncate (Variables|Default|GetTumblerRotation)) 180)
              (Variables|Default|SetTumblerNumber 5)
              (elif (== (Math|Float|Truncate (Variables|Default|GetTumblerRotation)) 216)
                (Variables|Default|SetTumblerNumber 6)
                (elif (== (Math|Float|Truncate (Variables|Default|GetTumblerRotation)) 252)
                  (Variables|Default|SetTumblerNumber 7)
                  (elif (== (Math|Float|Truncate (Variables|Default|GetTumblerRotation)) 288)
                    (Variables|Default|SetTumblerNumber 8)
                    (elif (== (Math|Float|Truncate (Variables|Default|GetTumblerRotation)) 324)
                      (Variables|Default|SetTumblerNumber 9)
                      (elif (== (Math|Float|Truncate (Variables|Default|GetTumblerRotation)) 360)
                        (Variables|Default|SetTumblerNumber 0)
                        (else
                          ;[1 1 1] Hacia atrás
                          (if (== (Math|Float|Truncate (Variables|Default|GetTumblerRotation)) -36)
                            (Variables|Default|SetTumblerNumber 9)
                            (elif (== (Math|Float|Truncate (Variables|Default|GetTumblerRotation)) -72)
                              (Variables|Default|SetTumblerNumber 8)
                              (elif (== (Math|Float|Truncate (Variables|Default|GetTumblerRotation)) -108)
                                (Variables|Default|SetTumblerNumber 7)
                                (elif (== (Math|Float|Truncate (Variables|Default|GetTumblerRotation)) -144)
                                  (Variables|Default|SetTumblerNumber 6)
                                  (elif (== (Math|Float|Truncate (Variables|Default|GetTumblerRotation)) -180)
                                    (Variables|Default|SetTumblerNumber 5)
                                    (elif (== (Math|Float|Truncate (Variables|Default|GetTumblerRotation)) -216)
                                      (Variables|Default|SetTumblerNumber 4)
                                      (elif (== (Math|Float|Truncate (Variables|Default|GetTumblerRotation)) -252)
                                        (Variables|Default|SetTumblerNumber 3)
                                        (elif (== (Math|Float|Truncate (Variables|Default|GetTumblerRotation)) -288)
                                          (Variables|Default|SetTumblerNumber 2)
                                          (elif (== (Math|Float|Truncate (Variables|Default|GetTumblerRotation)) -324)
                                            (Variables|Default|SetTumblerNumber 1)
                                            (elif (== (Math|Float|Truncate (Variables|Default|GetTumblerRotation)) -360)
                                              (Variables|Default|SetTumblerNumber 0))))))))))))))))))))))))

(fn RandomnizeTumbler
  (bind _randomrotations (Variables|Default|GetRandomRotations))
  (bind _output_get (Variables|Default|SetTumblerRotation (Utilities|Array|Get(acopy) _randomrotations (Math|Random|RandomIntegerinRange 0 (- (Utilities|Array|Length _randomrotations) 1)))))
  (Transformation|SetRelativeRotation (Variables|Default|GetTumblerMesh) (Math|Rotator|MakeRotator _output_get 0.0 0.0) false false)
  (CallFunction|NumberCheck))