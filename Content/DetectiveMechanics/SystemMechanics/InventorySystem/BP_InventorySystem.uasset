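; Inventory system Blueprint that stores item structures in a slot-indexed Inventory array.
; FindEmptySlot returns the first slot whose ItemName is "None", and SetSlot writes an item to a given index.
; Give looks up an ID in the Item_Data table and caches the row as Item, returning false if missing.
; Give is unfinished: its Items lookup leads nowhere and it never places the item in a slot.
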(fn FindEmptySlot
  (for (_array_element _array_index) (Variables|Default|GetInventory)
    (if (== (.itemname _array_element) "")
      (return true _array_index)))
  (return false 0))

(fn SetSlot
  (params (Slot :type Integer) (Item :type Item%20Structure%20Structure%20%28by%20ref%29))
  (Utilities|Array|SetArrayElem (Variables|Default|GetInventory) Slot Item))

(fn Give
  (params (ID :type Name))
  (Utilities|FlowControl|Sequence
    (:then_0
      (bind _returnvalue (Utilities|GetDataTableRow "/Game/DetectiveMechanics/SystemMechanics/InventorySystem/Item_Data.Item_Data" ID)
        (:then
          (bind _output_get (LocalVariables|SetItem _returnvalue))
          (bind _structout (Utilities|Struct|SetmembersinItemStructure _output_get))
          (LocalVariables|SetItem _structout))
        (:RowNotFound
          (return false))))
    (:then_1
      (if (.ReturnValue (Utilities|Map|Find (Variables|Default|GetItems) ID))
        _))))